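; Hand control Blueprint that rotates a finger phalanx (Falange) from a UI widget and sends the pose over a serial port.
; BeginPlay enables input, takes the SerialPort from GI_handBlueprint and binds the BPW_interfazHand rotation event.
; Each change sets the phalanx yaw, scales it into Pos, serializes that struct to bytes and writes them after a flush.
; Tick polls the port and prints incoming strings or a no-message notice.
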(event `self.ReceiveBeginPlay`
  (bind _returnvalue (`GameplayStatics.GetPlayerController` 0))
  (`|ExecutionSequence`
    (:`then_0`
      (`self.EnableInput` _returnvalue))
    (:`then_1`
      (bind _asgi_hand_blueprint (cast `/Game/Blueprints/GI_handBlueprint` (`GameplayStatics.GetGameInstance`)))
      (set `self.Serial Port` (`/Game/Blueprints/GI_handBlueprint.SerialPort` _asgi_hand_blueprint)))
    (:`then_2`
      (`EnhancedInputSubsystemInterface.AddMappingContext` (pcsubsystem `EnhancedInputLocalPlayerSubsystem` _returnvalue) null 0 (struct)))
    (:`then_3`
      (bind _returnvalue_2 (`|CreateWidget` "/Game/Blueprints/widgets/BPW_interfazHand.BPW_interfazHand_C"))
      (`UserWidget.AddToViewport` _returnvalue_2 0)
      (bind _output_get (set `self.interfaz` _returnvalue_2))
      (add `/Game/Blueprints/widgets/BPW_interfazHand.changeRotation1` _output_get (delegate `changeRotation`)))))

(event `changeRotation`
  (bind (_relativerotation_roll _relativerotation_pitch _relativerotation_yaw) (`KismetMathLibrary.BreakRotator` (`SceneComponent.RelativeRotation` (`self.falange`))))
  (`SceneComponent.K2_SetRelativeRotation` (`self.falange`) (`KismetMathLibrary.MakeRotator` 180.0 0.0 (`/Game/Blueprints/widgets/BPW_interfazHand.rotacion1` (`self.interfaz`))) false false)
  (set `self.pos` (make `Posiciones` (/ (* _relativerotation_yaw 180.0) 90.0)))
  (bind _newparam (`self.getBytes`))
  ; hay que activar el plugin pero primero hacer los cambios en c++ que sino se rompe.
  (`SerialCom.Flush` (`self.Serial Port`))
  (`SerialCom.WriteBytes` (`self.Serial Port`) _newparam))

(event `self.ReceiveTick`
  (params (DeltaSeconds :type "Float (single-precision)"))
  (bind (_bsuccess _returnvalue) (`SerialCom.ReadString` (`self.Serial Port`)))
  (if _bsuccess
    (`KismetSystemLibrary.PrintString` _returnvalue)
    (else
      (`KismetSystemLibrary.PrintString` "no hay mensaje"))))

(fn `getBytes`
  (returns (NewParam :type "Array of Byte"))
  (bind _returnvalue (`self.StructureToBytes` (`self.pos`)))
  (return _returnvalue))

(fn `UserConstructionScript`)