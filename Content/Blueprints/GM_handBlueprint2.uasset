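; GM_handBlueprint2, apparently a Game Mode, polls network calls on GI_handBlueprint and sets up mouse-driven UI input.
; BeginPlay switches the first player to UI-only input and shows the cursor; the widget creation nodes are disconnected.
; Every Tick casts the Game Instance, then accepts connections and receives a number as server.
; A hardcoded true branch leaves the client receive path unreachable.
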(event `self.ReceiveTick`
  (params (DeltaSeconds :type "Float (single-precision)"))
  (bind _asgi_hand_blueprint (cast `/Game/Blueprints/GI_handBlueprint` (`GameplayStatics.GetGameInstance`)))
  (set `self.As GI Hand Blueprint` _asgi_hand_blueprint)
  (if true
    (`GI_hand.aceptarConexion` (`self.As GI Hand Blueprint`))
    (`GI_hand.serverRecibirNumero` (`self.As GI Hand Blueprint`))
    (else
      (bind _returnvalue (`GI_hand.isClient` (`self.As GI Hand Blueprint`)))
      (if _returnvalue
        (`GI_hand.clientRecibirNumero` (`self.As GI Hand Blueprint`))))))

(event `self.ReceiveBeginPlay`
  (bind _returnvalue (`GameplayStatics.GetPlayerController` 0))
  (`WidgetBlueprintLibrary.SetInputMode_UIOnlyEx` _returnvalue null)
  (set `PlayerController.bShowMouseCursor` true _returnvalue))

(fn `UserConstructionScript`)