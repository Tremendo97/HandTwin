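; Free-fly camera Blueprint that also creates the BPW_menu widget on BeginPlay and reloads its serial port list.
; Enhanced Input drives swept movement along the camera's axes, rotation scaled by sensitivity, and FOV-based zoom, all frame-time scaled.
; Holding IA_switchMappings swaps IM_inputMap for IM_camera until release.
; Sensitivity, speed and FOV are written to GI_handBlueprint at startup, with FOV rewritten on each zoom.
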(event `self.ReceiveBeginPlay`
  (`|ExecutionSequence`
    (:`then_0`
      ; creamos y añadimos el menu
      (bind _returnvalue (`|CreateWidget` "/Game/Blueprints/widgets/BPW_menu.BPW_menu_C" (`GameplayStatics.GetPlayerController` 0)))
      (`UserWidget.AddToViewport` _returnvalue 0)
      (bind _output_get (set `self.menu` _returnvalue))
      ; recargamos los serial ports
      (`/Game/Blueprints/widgets/BPW_menu.recargarSerialPorts` _output_get))
    (:`then_1`
      (bind _asgi_hand_blueprint (cast `/Game/Blueprints/GI_handBlueprint` (`GameplayStatics.GetGameInstance`)))
      (`/Game/Blueprints/GI_handBlueprint.setControles` _asgi_hand_blueprint "NewEnumerator0" (`self.sensibilidad`))
      (`/Game/Blueprints/GI_handBlueprint.setControles` _asgi_hand_blueprint "NewEnumerator2" (`self.velocidadCamara`))
      (`/Game/Blueprints/GI_handBlueprint.setControles` _asgi_hand_blueprint "NewEnumerator1" (`CameraComponent.FieldOfView` (`self.Camera`))))))

(event `EnhancedInput|/Game/Blueprints/input/camera/IA_zoomIn`
  (params (ActionValue :type "Float (double-precision)") (ElapsedSeconds :type "Float (double-precision)") (TriggeredSeconds :type "Float (double-precision)") (InputAction :type "InputAction Object Reference" :default "/Game/Blueprints/input/camera/IA_zoomIn.IA_zoomIn"))
  ; zoom
  (:`Triggered`
    (`self.zoom` ActionValue)))

(event `EnhancedInput|/Game/Blueprints/input/camera/IA_moveForward`
  (params (ActionValue :type Boolean) (ElapsedSeconds :type "Float (double-precision)") (TriggeredSeconds :type "Float (double-precision)") (InputAction :type "InputAction Object Reference" :default "/Game/Blueprints/input/camera/IA_moveForward.IA_moveForward"))
  ; movieminto de la camara
  (:`Triggered`
    (`self.K2_SetActorLocation` (+ (`self.K2_GetActorLocation`) (* (`SceneComponent.GetForwardVector` (`self.Camera`)) (* (`GameplayStatics.GetWorldDeltaSeconds`) (`self.velocidadCamara`)))) true)))

(event `EnhancedInput|/Game/Blueprints/input/camera/IA_moveReverse`
  (params (ActionValue :type Boolean) (ElapsedSeconds :type "Float (double-precision)") (TriggeredSeconds :type "Float (double-precision)") (InputAction :type "InputAction Object Reference" :default "/Game/Blueprints/input/camera/IA_moveReverse.IA_moveReverse"))
  ; movieminto de la camara
  (:`Triggered`
    (`self.K2_SetActorLocation` (- (`self.K2_GetActorLocation`) (* (`SceneComponent.GetForwardVector` (`self.Camera`)) (* (`GameplayStatics.GetWorldDeltaSeconds`) (`self.velocidadCamara`)))) true)))

(event `EnhancedInput|/Game/Blueprints/input/camera/IA_moveRight`
  (params (ActionValue :type Boolean) (ElapsedSeconds :type "Float (double-precision)") (TriggeredSeconds :type "Float (double-precision)") (InputAction :type "InputAction Object Reference" :default "/Game/Blueprints/input/camera/IA_moveRight.IA_moveRight"))
  ; movieminto de la camara
  (:`Triggered`
    (`self.K2_SetActorLocation` (+ (`self.K2_GetActorLocation`) (* (`SceneComponent.GetRightVector` (`self.Camera`)) (* (`GameplayStatics.GetWorldDeltaSeconds`) (`self.velocidadCamara`)))) true)))

(event `EnhancedInput|/Game/Blueprints/input/camera/IA_moveLeft`
  (params (ActionValue :type Boolean) (ElapsedSeconds :type "Float (double-precision)") (TriggeredSeconds :type "Float (double-precision)") (InputAction :type "InputAction Object Reference" :default "/Game/Blueprints/input/camera/IA_moveLeft.IA_moveLeft"))
  ; movieminto de la camara
  (:`Triggered`
    (`self.K2_SetActorLocation` (- (`self.K2_GetActorLocation`) (* (`SceneComponent.GetRightVector` (`self.Camera`)) (* (`GameplayStatics.GetWorldDeltaSeconds`) (`self.velocidadCamara`)))) true)))

(event `EnhancedInput|/Game/Blueprints/input/IA_switchMappings`
  (params (ActionValue :type Boolean) (ElapsedSeconds :type "Float (double-precision)") (TriggeredSeconds :type "Float (double-precision)") (InputAction :type "InputAction Object Reference" :default "/Game/Blueprints/input/IA_switchMappings.IA_switchMappings"))
  (bind _returnvalue (pcsubsystem `EnhancedInputLocalPlayerSubsystem` (`GameplayStatics.GetPlayerController` 0)))
  (bind _returnvalue_2 (pcsubsystem `EnhancedInputLocalPlayerSubsystem` (`GameplayStatics.GetPlayerController` 0)))
  ; Cambio del input mapping
  (:`Started`
    (`EnhancedInputSubsystemInterface.RemoveMappingContext` _returnvalue "/Game/Blueprints/input/hand/IM_inputMap.IM_inputMap" (struct))
    (`EnhancedInputSubsystemInterface.AddMappingContext` _returnvalue "/Game/Blueprints/input/camera/IM_camera.IM_camera" 0 (struct)))
  (:`Canceled`
    (`EnhancedInputSubsystemInterface.RemoveMappingContext` _returnvalue_2 "/Game/Blueprints/input/camera/IM_camera.IM_camera" (struct) :!label _label)
    (`EnhancedInputSubsystemInterface.AddMappingContext` _returnvalue_2 "/Game/Blueprints/input/hand/IM_inputMap.IM_inputMap" 0 (struct)))
  (:`Completed`
    (goto _label)))

(event `EnhancedInput|/Game/Blueprints/input/camera/IA_turnCamera_panCamera`
  (params (ActionValue :type "Vector2D Structure") (ElapsedSeconds :type "Float (double-precision)") (TriggeredSeconds :type "Float (double-precision)") (InputAction :type "InputAction Object Reference" :default "/Game/Blueprints/input/camera/IA_turnCamera_panCamera.IA_turnCamera_panCamera"))
  (bind _returnvalue (`GameplayStatics.GetWorldDeltaSeconds`))
  (bind _sensibilidad (`self.sensibilidad`))
  ; rotacion de la camara
  (:`Triggered`
    (`SceneComponent.K2_AddRelativeRotation` (`self.Camera`) (`KismetMathLibrary.MakeRotator` 0.0 (* (* ActionValue_Y _sensibilidad) _returnvalue) (* (* ActionValue_X _sensibilidad) _returnvalue)) false false)))

(event `self.ReceiveTick`
  (params (DeltaSeconds :type "Float (single-precision)")))

(fn `UserConstructionScript`)

(fn `zoom`
  (params (NewParam :type "Float (double-precision)"))
  (`CameraComponent.SetFieldOfView` (`self.Camera`) (+ (* (* NewParam 100.0) (`GameplayStatics.GetWorldDeltaSeconds`)) (`CameraComponent.FieldOfView` (`self.Camera`))))
  (bind _asgi_hand_blueprint (cast `/Game/Blueprints/GI_handBlueprint` (`GameplayStatics.GetGameInstance`)))
  (`/Game/Blueprints/GI_handBlueprint.setControles` _asgi_hand_blueprint "NewEnumerator1" (`CameraComponent.FieldOfView` (`self.Camera`))))