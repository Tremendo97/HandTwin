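; Game instance that owns the serial port connection and keeps it available across the game's lifetime.
; RecargarSerialPorts returns the available ports and also runs on Init, while SetSerialPort opens a chosen port at a fixed baud rate, stores it and broadcasts SerialPortChanged.
; On Shutdown, a valid port is closed and CloseAplication is called, which a comment describes as unused socket cleanup.
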(event `self.ReceiveInit`
  (`self.RecargarSerialPorts`))

(event `self.ReceiveShutdown`
  (`/Engine/EditorBlueprintResources/StandardMacros.IsValid` (`self.SerialPort`)
    (:`Is Valid`
      ; cerramos el puerto serial
      (`SerialCom.Close` (`self.SerialPort`))
      ; cerrar sockets pero no se usa
      (`self.closeAplication`))))

(fn `RecargarSerialPorts`
  (returns (NewParam :type "Map of Integer to String"))
  (bind _returnvalue (`FL_hand2.getAvailablePorts`))
  (return _returnvalue))

(fn `setSerialPort`
  (params (serialPort :type Integer))
  ; Open serial port
  (bind (_bopened _returnvalue) (`SerialCom.OpenComPort` serialPort))
  (set `self.SerialPort` _returnvalue)
  (`self.serialPortChanged`))