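; BP_finger is one finger of a virtual hand that mirrors its joint pose to a serial device.
; Flex/extend events rotate phalanges at frame-rate-independent speed within clamped limits, with one angle driving the two outer joints sequentially.
; Yaws are rescaled into a structure with the finger ID, then written as bytes to GI_handBlueprint's serial port only on change.
; It also registers the input mapping context and swaps materials to show active state.
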(event `self.ReceiveBeginPlay`
  (`|ExecutionSequence`
    (:`then_0`
      ; activar el input en el blueprint
      (`self.EnableInput` (`GameplayStatics.GetPlayerController` 0)))
    (:`then_1`
      (`EnhancedInputSubsystemInterface.AddMappingContext` (pcsubsystem `EnhancedInputLocalPlayerSubsystem` (`GameplayStatics.GetPlayerController` 0)) "/Game/Blueprints/input/hand/IM_inputMap.IM_inputMap" 0 (struct)))
    (:`then_2`
      (bind _asgi_hand_blueprint (cast `/Game/Blueprints/GI_handBlueprint` (`GameplayStatics.GetGameInstance`)))
      (add `/Game/Blueprints/GI_handBlueprint.serialPortChanged` _asgi_hand_blueprint (delegate `setSerialPort`)))))

(event `setSerialPort`
  ; set serial port, se ejecuta cuando cambia en el game instance
  (bind _asgi_hand_blueprint (cast `/Game/Blueprints/GI_handBlueprint` (`GameplayStatics.GetGameInstance`)))
  (set `self.Serial Port` (`/Game/Blueprints/GI_handBlueprint.SerialPort` _asgi_hand_blueprint))
  (`KismetSystemLibrary.PrintString` (`KismetStringLibrary.Concat_StrStr` "se cambia el serial port desde el " (`|GetEnumeratorNameAsString` (`self.dedo`)))))

(event `flexFalange1`
  (bind (_relativerotation_roll _relativerotation_pitch _relativerotation_yaw) (`KismetMathLibrary.BreakRotator` (`SceneComponent.RelativeRotation` (`self.falange`))))
  (`self.rotarPrimeraArticulacion` (`self.falange`) (- _relativerotation_yaw (* (`self.velocidad`) (`GameplayStatics.GetWorldDeltaSeconds`))))
  (`self.SetPosEstructure` :!label _label)
  (`self.enviarPuertoSerie`))

(event `extFalange1`
  (bind (_relativerotation_roll _relativerotation_pitch _relativerotation_yaw) (`KismetMathLibrary.BreakRotator` (`SceneComponent.RelativeRotation` (`self.falange`))))
  (`self.rotarPrimeraArticulacion` (`self.falange`) (+ _relativerotation_yaw (* (`self.velocidad`) (`GameplayStatics.GetWorldDeltaSeconds`))))
  (goto _label))

(event `flexFalange2`
  (bind (_relativerotation_roll _relativerotation_pitch _relativerotation_yaw) (`KismetMathLibrary.BreakRotator` (`SceneComponent.RelativeRotation` (`self.falange1`))))
  (bind (_relativerotation_roll_2 _relativerotation_pitch_2 _relativerotation_yaw_2) (`KismetMathLibrary.BreakRotator` (`SceneComponent.RelativeRotation` (`self.falange2`))))
  (`self.rotarSegundaArticulacion` (`self.falange1`) (`self.falange2`) (- (/ (+ _relativerotation_yaw _relativerotation_yaw_2) 2.0) (* (`self.velocidad`) (`GameplayStatics.GetWorldDeltaSeconds`))))
  (goto _label))

(event `extFalange2`
  (bind (_relativerotation_roll _relativerotation_pitch _relativerotation_yaw) (`KismetMathLibrary.BreakRotator` (`SceneComponent.RelativeRotation` (`self.falange1`))))
  (bind (_relativerotation_roll_2 _relativerotation_pitch_2 _relativerotation_yaw_2) (`KismetMathLibrary.BreakRotator` (`SceneComponent.RelativeRotation` (`self.falange2`))))
  (`self.rotarSegundaArticulacion` (`self.falange1`) (`self.falange2`) (+ (/ (+ _relativerotation_yaw _relativerotation_yaw_2) 2.0) (* (`self.velocidad`) (`GameplayStatics.GetWorldDeltaSeconds`))))
  (goto _label))

(fn `enviarPuertoSerie`
  (`/Engine/EditorBlueprintResources/StandardMacros.IsValid` (`self.Serial Port`)
    (:`Is Valid`
      (bind _returnvalue (`FL_hand2.EqualStructure` (`self.pos`) (`self.posAnterior`)))
      (if (not _returnvalue)
        ; enviar a traves del puerto serie
        (bind _returnvalue_2 (`FL_hand2.StructureToBytes` (`self.pos`)))
        (`SerialCom.Flush` (`self.Serial Port`))
        (`SerialCom.WriteBytes` (`self.Serial Port`) _returnvalue_2)
        (bind _output_get (set `self.posAnterior` (`self.pos`)))
        (`KismetSystemLibrary.PrintString` (`KismetStringLibrary.Conv_DoubleToString` (break `Posiciones` _output_get)))))
    (:`Is Not Valid`
      (`KismetSystemLibrary.PrintString` "el puerto no es valido "))))

(fn `rotarPrimeraArticulacion`
  (params (Falange1 :type "StaticMeshComponent Object Reference") (angulo :type "Float (double-precision)"))
  (bind (_relativerotation_roll _relativerotation_pitch) (`KismetMathLibrary.BreakRotator` (`SceneComponent.RelativeRotation` (`local.Falange1`))))
  (bind (_relativerotation_roll_2 _relativerotation_pitch_2) (`KismetMathLibrary.BreakRotator` (`SceneComponent.RelativeRotation` (`local.Falange1`))))
  (if (> angulo 0.0)
    (`SceneComponent.K2_SetRelativeRotation` (`local.Falange1`) (`KismetMathLibrary.MakeRotator` _relativerotation_roll_2 _relativerotation_pitch_2) false false)
    (elif (< (`local.angulo`) -90.0)
      (`SceneComponent.K2_SetRelativeRotation` (`local.Falange1`) (`KismetMathLibrary.MakeRotator` _relativerotation_roll _relativerotation_pitch -90.0) false false)
      (else
        (`SceneComponent.K2_SetRelativeRotation` (`local.Falange1`) (`KismetMathLibrary.MakeRotator` _relativerotation_roll _relativerotation_pitch (`local.angulo`)) false false)))))

(fn `rotarSegundaArticulacion`
  (params (falange2 :type "StaticMeshComponent Object Reference") (falange3 :type "StaticMeshComponent Object Reference") (angulo :type "Float (double-precision)"))
  (locals (falange2XY :type "Vector2D Structure") (falange3XY :type "Vector2D Structure"))
  (bind (_relativerotation_roll _relativerotation_pitch) (`KismetMathLibrary.BreakRotator` (`SceneComponent.RelativeRotation` falange2)))
  (bind (_falange2xy_x _falange2xy_y) (`KismetMathLibrary.BreakVector2D` (`local.falange2XY`)))
  (bind (_falange3xy_x _falange3xy_y) (`KismetMathLibrary.BreakVector2D` (`local.falange3XY`)))
  (bind (_falange2xy_x_2 _falange2xy_y_2) (`KismetMathLibrary.BreakVector2D` (`local.falange2XY`)))
  (bind (_falange3xy_x_2 _falange3xy_y_2) (`KismetMathLibrary.BreakVector2D` (`local.falange3XY`)))
  (bind (_falange2xy_x_3 _falange2xy_y_3) (`KismetMathLibrary.BreakVector2D` (`local.falange2XY`)))
  (bind (_falange3xy_x_3 _falange3xy_y_3) (`KismetMathLibrary.BreakVector2D` (`local.falange3XY`)))
  (bind (_falange2xy_x_4 _falange2xy_y_4) (`KismetMathLibrary.BreakVector2D` (`local.falange2XY`)))
  (bind (_falange3xy_x_4 _falange3xy_y_4) (`KismetMathLibrary.BreakVector2D` (`local.falange3XY`)))
  (bind (_relativerotation_roll_2 _relativerotation_pitch_2) (`KismetMathLibrary.BreakRotator` (`SceneComponent.RelativeRotation` falange3)))
  (set `local.falange2XY` (`KismetMathLibrary.MakeVector2D` _relativerotation_roll _relativerotation_pitch))
  (set `local.falange3XY` (`KismetMathLibrary.MakeVector2D` _relativerotation_roll_2 _relativerotation_pitch_2))
  (if (> (`local.angulo`) -7.0)
    (`SceneComponent.K2_SetRelativeRotation` (`local.falange2`) (`KismetMathLibrary.MakeRotator` _falange2xy_x_2 _falange2xy_y_2 -7.0) false false)
    (`SceneComponent.K2_SetRelativeRotation` (`local.falange3`) (`KismetMathLibrary.MakeRotator` _falange3xy_x_2 _falange3xy_y_2 -7.0) false false)
    (elif (< (`local.angulo`) -70.0)
      (`SceneComponent.K2_SetRelativeRotation` (`local.falange2`) (`KismetMathLibrary.MakeRotator` _falange2xy_x_3 _falange2xy_y_3 -70.0) false false)
      (`SceneComponent.K2_SetRelativeRotation` (`local.falange3`) (`KismetMathLibrary.MakeRotator` _falange3xy_x_3 _falange3xy_y_3 -70.0) false false)
      (elif (> (`local.angulo`) -35.0)
        (`SceneComponent.K2_SetRelativeRotation` (`local.falange3`) (`KismetMathLibrary.MakeRotator` _falange2xy_x_4 _falange2xy_y_4 (* (`local.angulo`) 2.0)) false false)
        (`SceneComponent.K2_SetRelativeRotation` (`local.falange2`) (`KismetMathLibrary.MakeRotator` _falange3xy_x_4 _falange3xy_y_4) false false)
        (else
          (`SceneComponent.K2_SetRelativeRotation` (`local.falange2`) (`KismetMathLibrary.MakeRotator` _falange2xy_x _falange2xy_y (* (+ (`local.angulo`) 35.0) 2.0)) false false)
          (`SceneComponent.K2_SetRelativeRotation` (`local.falange3`) (`KismetMathLibrary.MakeRotator` _falange3xy_x _falange3xy_y -70.0) false false))))))

(fn `setActiveFinger`
  (`PrimitiveComponent.SetMaterial` (`self.falange`) 0 "/Game/materials/M_mano_active.M_mano_active")
  (`PrimitiveComponent.SetMaterial` (`self.falange1`) 0 "/Game/materials/M_mano_active.M_mano_active")
  (`PrimitiveComponent.SetMaterial` (`self.falange2`) 0 "/Game/materials/M_mano_active.M_mano_active"))

(fn `setFinger`
  (params (dedo :type "EDedos Enum" :default "Indice"))
  (set `self.dedo` dedo))

(fn `SetPosEstructure`
  (bind (_relativerotation_roll _relativerotation_pitch _relativerotation_yaw) (`KismetMathLibrary.BreakRotator` (`SceneComponent.RelativeRotation` (`self.falange`))))
  (bind (_relativerotation_roll_2 _relativerotation_pitch_2 _relativerotation_yaw_2) (`KismetMathLibrary.BreakRotator` (`SceneComponent.RelativeRotation` (`self.falange1`))))
  (bind (_relativerotation_roll_3 _relativerotation_pitch_3 _relativerotation_yaw_3) (`KismetMathLibrary.BreakRotator` (`SceneComponent.RelativeRotation` (`self.falange2`))))
  (bind _newparam1 (`self.transformacionFalange1` _relativerotation_yaw))
  (bind _newparam1_2 (`self.transformacionFalange2` (/ (+ _relativerotation_yaw_2 _relativerotation_yaw_3) 2.0)))
  (set `self.pos` (make `Posiciones` _newparam1 _newparam1_2 (`self.dedo`))))

(fn `transformacionFalange1`
  (params (NewParam :type "Float (double-precision)"))
  (returns (NewParam1 :type "Float (double-precision)"))
  (return (- 0.0 (/ (* NewParam 150.0) 90.0))))

(fn `transformacionFalange2`
  (params (NewParam :type "Float (double-precision)"))
  (returns (NewParam1 :type "Float (double-precision)"))
  (return (- 0.0 (/ (* (+ NewParam 7.0) 180.0) 63.0))))

(fn `unActiveFinger`
  (`PrimitiveComponent.SetMaterial` (`self.falange`) 0 "/Game/materials/M_mano_inactive.M_mano_inactive")
  (`PrimitiveComponent.SetMaterial` (`self.falange1`) 0 "/Game/materials/M_mano_inactive.M_mano_inactive")
  (`PrimitiveComponent.SetMaterial` (`self.falange2`) 0 "/Game/materials/M_mano_inactive.M_mano_inactive"))

(fn `UserConstructionScript`)