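; BP_mano is a hand actor that lets the player select one finger at a time and flex or extend its two phalanges.
; On BeginPlay it enables input, gathers BP_finger child actors into an array, initializes each by component name and activates the one at index 1.
; Enhanced Input actions forward phalange movements to the active finger, while ChangeActiveFinger cycles the selection with wraparound.
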(event `self.ReceiveBeginPlay`
  (bind _output (`|GetArrayItem` (`self.dedos`) 1))
  (`|ExecutionSequence`
    (:`then_0`
      (`self.EnableInput` (`GameplayStatics.GetPlayerController` 0)))
    (:`then_1`
      (for _array_element (`SceneComponent.GetChildrenComponents` (`self.DefaultSceneRoot`) false)
        (bind _aschild_actor_component (cast `ChildActorComponent` _array_element))
        (bind _asbp_finger (cast `/Game/Blueprints/BP_finger` (`ChildActorComponent.ChildActor` _aschild_actor_component)))
        (`KismetArrayLibrary.Array_Add` (`self.dedos`) _asbp_finger)
        ; inicializamos cada uno de los dedos en funcion de su nombre
        (switch `string` (`KismetSystemLibrary.GetObjectName` _array_element)
          (:`anular`
            (`/Game/Blueprints/BP_finger.setFinger` _asbp_finger "Anular"))
          (:`corazon`
            (`/Game/Blueprints/BP_finger.setFinger` _asbp_finger "Corazon"))
          (:`menique`
            (`/Game/Blueprints/BP_finger.setFinger` _asbp_finger "Menique"))
          (:`indice`
            (`/Game/Blueprints/BP_finger.setFinger` _asbp_finger "Indice"))))
      (`/Game/Blueprints/BP_finger.setActiveFinger` _output)
      (set `self.activeFinger` _output))))

(event `EnhancedInput|/Game/Blueprints/input/hand/IA_flexFalange1`
  (params (ActionValue :type Boolean) (ElapsedSeconds :type "Float (double-precision)") (TriggeredSeconds :type "Float (double-precision)") (InputAction :type "InputAction Object Reference" :default "/Game/Blueprints/input/hand/IA_flexFalange1.IA_flexFalange1"))
  (:`Triggered`
    (`/Game/Blueprints/BP_finger.flexFalange1` (`self.activeFinger`))))

(event `EnhancedInput|/Game/Blueprints/input/hand/IA_extFalange1`
  (params (ActionValue :type Boolean) (ElapsedSeconds :type "Float (double-precision)") (TriggeredSeconds :type "Float (double-precision)") (InputAction :type "InputAction Object Reference" :default "/Game/Blueprints/input/hand/IA_extFalange1.IA_extFalange1"))
  (:`Triggered`
    (`/Game/Blueprints/BP_finger.extFalange1` (`self.activeFinger`))))

(event `EnhancedInput|/Game/Blueprints/input/hand/IA_flexFalange2`
  (params (ActionValue :type Boolean) (ElapsedSeconds :type "Float (double-precision)") (TriggeredSeconds :type "Float (double-precision)") (InputAction :type "InputAction Object Reference" :default "/Game/Blueprints/input/hand/IA_flexFalange2.IA_flexFalange2"))
  (:`Triggered`
    (`/Game/Blueprints/BP_finger.flexFalange2` (`self.activeFinger`))))

(event `EnhancedInput|/Game/Blueprints/input/hand/IA_extFalange2`
  (params (ActionValue :type Boolean) (ElapsedSeconds :type "Float (double-precision)") (TriggeredSeconds :type "Float (double-precision)") (InputAction :type "InputAction Object Reference" :default "/Game/Blueprints/input/hand/IA_extFalange2.IA_extFalange2"))
  (:`Triggered`
    (`/Game/Blueprints/BP_finger.extFalange2` (`self.activeFinger`))))

(event `EnhancedInput|/Game/Blueprints/input/hand/IA_changeLeftFinger`
  (params (ActionValue :type Boolean) (ElapsedSeconds :type "Float (double-precision)") (TriggeredSeconds :type "Float (double-precision)") (InputAction :type "InputAction Object Reference" :default "/Game/Blueprints/input/hand/IA_changeLeftFinger.IA_changeLeftFinger"))
  (:`Started`
    (`self.changeActiveFinger` false)))

(event `EnhancedInput|/Game/Blueprints/input/hand/IA_changeRightFinger`
  (params (ActionValue :type Boolean) (ElapsedSeconds :type "Float (double-precision)") (TriggeredSeconds :type "Float (double-precision)") (InputAction :type "InputAction Object Reference" :default "/Game/Blueprints/input/hand/IA_changeRightFinger.IA_changeRightFinger"))
  (:`Started`
    (`self.changeActiveFinger` true)))

(event `self.ReceiveTick`
  (params (DeltaSeconds :type "Float (single-precision)")))

(fn `changeActiveFinger`
  (params (direccion :type Boolean :default true))
  (bind _output (`|GetArrayItem` (`self.dedos`) (`self.indiceActiveFinger`)))
  (if direccion
    (bind _output_get (set `self.indiceActiveFinger` (+ -1 (`self.indiceActiveFinger`))))
    (if (< _output_get 0)
      (set `self.indiceActiveFinger` (- (`KismetArrayLibrary.Array_Length` (`self.dedos`)) 1)))
    (else
      (bind _output_get_2 (set `self.indiceActiveFinger` (+ 1 (`self.indiceActiveFinger`))))
      (if (>= _output_get_2 (`KismetArrayLibrary.Array_Length` (`self.dedos`)))
        (set `self.indiceActiveFinger` 0))))
  (`/Game/Blueprints/BP_finger.unActiveFinger` (`self.activeFinger`))
  (set `self.activeFinger` _output)
  (`/Game/Blueprints/BP_finger.setActiveFinger` _output))

(fn `UserConstructionScript`)