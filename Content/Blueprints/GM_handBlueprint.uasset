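; GM_handBlueprint, apparently a game mode, sets up mouse-driven UI input and polls a networked number exchange.
; BeginPlay shows the cursor and sets UI-only input for player 0.
; Each Tick casts the GameInstance and calls it by role: servers accept connections and receive a number, clients only receive one.
; Widget creation and a duplicate input setup remain as unconnected nodes.
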(event `self.ReceiveTick`
  (params (DeltaSeconds :type "Float (single-precision)"))
  (bind _asgi_hand_blueprint (cast `` (`GameplayStatics.GetGameInstance` null)))
  (if (`KismetSystemLibrary.IsServer` _asgi_hand_blueprint null)
    (`self.aceptarConexion` _asgi_hand_blueprint)
    (`self.serverRecibirNumero` _asgi_hand_blueprint)
    (else
      (bind _returnvalue (`self.isClient` _asgi_hand_blueprint))
      (if _returnvalue
        (`self.clientRecibirNumero` _asgi_hand_blueprint)))))

(event `self.ReceiveBeginPlay`
  (bind _returnvalue (`GameplayStatics.GetPlayerController` null))
  (`WidgetBlueprintLibrary.SetInputMode_UIOnlyEx` _returnvalue null)
  (set `PlayerController.bShowMouseCursor` true _returnvalue))

(fn `UserConstructionScript`)