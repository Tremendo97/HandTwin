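; BP_mano is a player-controlled hand that manages five BP_finger child actors, with one active at a time.
; On BeginPlay it identifies the fingers under Palma by component name and stores them in Dedos.
; Input cycles the active finger, flexes or extends its two phalanges, and adjusts a clamped Velocidad.
; Velocidad syncs through GI_handBlueprint's controls-changed event; an Arduino serial read exists but never runs.
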(event `self.ReceiveBeginPlay`
  (bind _output (`|GetArrayItem` (`self.dedos`)))
  (`|ExecutionSequence`
    (:`then_0`
      (`self.EnableInput` (`GameplayStatics.GetPlayerController` 0)))
    (:`then_1`
      (for _array_element (`SceneComponent.GetChildrenComponents` (`self.palma`) false)
        (bind _aschild_actor_component (cast `ChildActorComponent` _array_element))
        (bind _asbp_finger (cast `/Game/Blueprints/hand/BP_finger` (`ChildActorComponent.ChildActor` _aschild_actor_component)))
        ; inicializamos cada uno de los dedos en funcion de su nombre
        (switch `string` (`KismetSystemLibrary.GetObjectName` _array_element)
          (:`anular`
            (`/Game/Blueprints/hand/BP_finger.setFinger` _asbp_finger "Anular")
            (`KismetArrayLibrary.Array_Set` (`self.dedos`) 1 _asbp_finger))
          (:`corazon`
            (`/Game/Blueprints/hand/BP_finger.setFinger` _asbp_finger "Corazon")
            (`KismetArrayLibrary.Array_Set` (`self.dedos`) 2 _asbp_finger))
          (:`menique`
            (`/Game/Blueprints/hand/BP_finger.setFinger` _asbp_finger "Menique")
            (`KismetArrayLibrary.Array_Set` (`self.dedos`) 0 _asbp_finger))
          (:`indice`
            (`/Game/Blueprints/hand/BP_finger.setFinger` _asbp_finger "Indice")
            (`KismetArrayLibrary.Array_Set` (`self.dedos`) 3 _asbp_finger))
          (:`pulgar`
            (`/Game/Blueprints/hand/BP_finger.setFinger` _asbp_finger "Pulgar")
            (`KismetArrayLibrary.Array_Set` (`self.dedos`) 4 _asbp_finger))))
      (`/Game/Blueprints/hand/BP_finger.setActiveFinger` _output)
      (set `self.activeFinger` _output))
    (:`then_2`
      (bind _asgi_hand_blueprint (cast `/Game/Blueprints/GI_handBlueprint` (`GameplayStatics.GetGameInstance`)))
      (`/Game/Blueprints/GI_handBlueprint.setControles` _asgi_hand_blueprint "NewEnumerator3" (`self.velocidad`))
      (add `/Game/Blueprints/GI_handBlueprint.controlesChanged` _asgi_hand_blueprint (delegate `CustomEvent`)))))

(event `CustomEvent`
  (params (parametro :type "/Game/Estructuras/ENUM_controlesParameters Enum" :default "NewEnumerator0") (valor :type "Float (double-precision)"))
  (if (== parametro 3)
    (set `self.velocidad` valor)))

(event `EnhancedInput|/Game/Blueprints/input/hand/IA_changeLeftFinger`
  (params (ActionValue :type Boolean) (ElapsedSeconds :type "Float (double-precision)") (TriggeredSeconds :type "Float (double-precision)") (InputAction :type "InputAction Object Reference" :default "/Game/Blueprints/input/hand/IA_changeLeftFinger.IA_changeLeftFinger"))
  ; cambia el dedo activo
  (:`Started`
    (`self.changeActiveFinger` false)))

(event `EnhancedInput|/Game/Blueprints/input/hand/IA_flexFalange1`
  (params (ActionValue :type Boolean) (ElapsedSeconds :type "Float (double-precision)") (TriggeredSeconds :type "Float (double-precision)") (InputAction :type "InputAction Object Reference" :default "/Game/Blueprints/input/hand/IA_flexFalange1.IA_flexFalange1"))
  ; felxion y extension del dedo activo
  (:`Triggered`
    (`/Game/Blueprints/hand/BP_finger.flexFalange1` (`self.activeFinger`))))

(event `EnhancedInput|/Game/Blueprints/input/hand/IA_changeRightFinger`
  (params (ActionValue :type Boolean) (ElapsedSeconds :type "Float (double-precision)") (TriggeredSeconds :type "Float (double-precision)") (InputAction :type "InputAction Object Reference" :default "/Game/Blueprints/input/hand/IA_changeRightFinger.IA_changeRightFinger"))
  ; cambia el dedo activo
  (:`Started`
    (`self.changeActiveFinger` true)))

(event `EnhancedInput|/Game/Blueprints/input/hand/IA_extFalange1`
  (params (ActionValue :type Boolean) (ElapsedSeconds :type "Float (double-precision)") (TriggeredSeconds :type "Float (double-precision)") (InputAction :type "InputAction Object Reference" :default "/Game/Blueprints/input/hand/IA_extFalange1.IA_extFalange1"))
  ; felxion y extension del dedo activo
  (:`Triggered`
    (`/Game/Blueprints/hand/BP_finger.extFalange1` (`self.activeFinger`))))

(event `EnhancedInput|/Game/Blueprints/input/hand/IA_flexFalange2`
  (params (ActionValue :type Boolean) (ElapsedSeconds :type "Float (double-precision)") (TriggeredSeconds :type "Float (double-precision)") (InputAction :type "InputAction Object Reference" :default "/Game/Blueprints/input/hand/IA_flexFalange2.IA_flexFalange2"))
  ; felxion y extension del dedo activo
  (:`Triggered`
    (`/Game/Blueprints/hand/BP_finger.flexFalange2` (`self.activeFinger`))))

(event `EnhancedInput|/Game/Blueprints/input/hand/IA_extFalange2`
  (params (ActionValue :type Boolean) (ElapsedSeconds :type "Float (double-precision)") (TriggeredSeconds :type "Float (double-precision)") (InputAction :type "InputAction Object Reference" :default "/Game/Blueprints/input/hand/IA_extFalange2.IA_extFalange2"))
  ; felxion y extension del dedo activo
  (:`Triggered`
    (`/Game/Blueprints/hand/BP_finger.extFalange2` (`self.activeFinger`))))

(event `self.ReceiveTick`
  (params (DeltaSeconds :type "Float (single-precision)")))

(event `EnhancedInput|/Game/Blueprints/input/hand/IA_changeVelocidad`
  (params (ActionValue :type "Float (double-precision)") (ElapsedSeconds :type "Float (double-precision)") (TriggeredSeconds :type "Float (double-precision)") (InputAction :type "InputAction Object Reference" :default "/Game/Blueprints/input/hand/IA_changeVelocidad.IA_changeVelocidad"))
  (bind _returnvalue (+ (* ActionValue 10.0) (`self.velocidad`)))
  (:`Triggered`
    (if (<= _returnvalue 0.0)
      (set `self.velocidad` 0.0)
      (elif (>= _returnvalue 242.424)
        (set `self.velocidad` 242.424)
        (else
          (set `self.velocidad` _returnvalue))))
    ; avisamos que al game instance que la velocidad cambio
    (bind _asgi_hand_blueprint (cast `/Game/Blueprints/GI_handBlueprint` (`GameplayStatics.GetGameInstance`)))
    (`/Game/Blueprints/GI_handBlueprint.setControles` _asgi_hand_blueprint "NewEnumerator3" (`self.velocidad`))))

(fn `changeActiveFinger`
  (params (direccion :type Boolean :default true))
  (bind _output (`|GetArrayItem` (`self.dedos`) (`self.indiceActiveFinger`)))
  (if direccion
    (bind _output_get (set `self.indiceActiveFinger` (+ -1 (`self.indiceActiveFinger`))))
    (if (< _output_get 0)
      (set `self.indiceActiveFinger` (- (`KismetArrayLibrary.Array_Length` (`self.dedos`)) 1)))
    (else
      (bind _output_get_2 (set `self.indiceActiveFinger` (+ 1 (`self.indiceActiveFinger`))))
      (if (>= _output_get_2 (`KismetArrayLibrary.Array_Length` (`self.dedos`)))
        (set `self.indiceActiveFinger` 0))))
  (`/Game/Blueprints/hand/BP_finger.unActiveFinger` (`self.activeFinger`))
  (set `self.activeFinger` _output)
  (`/Game/Blueprints/hand/BP_finger.setActiveFinger` _output))

(fn `setActiveFinger`
  (params (newActiveFinger :type "ChildActorComponent Object Reference"))
  (bind _asbp_finger (cast `/Game/Blueprints/hand/BP_finger` (`ChildActorComponent.ChildActor` newActiveFinger)))
  (`/Game/Blueprints/hand/BP_finger.setActiveFinger` _asbp_finger)
  (set `self.activeFinger` _asbp_finger))

(fn `UserConstructionScript`)