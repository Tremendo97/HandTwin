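; BP_pulgar is the thumb of a hand, a child Blueprint that specializes its parent finger's joint-to-pulley angle mapping.
; Rotating the first joint recomputes the second pulley's min and max limits from that angle before calling the parent.
; The second phalange's negated angle is clamp-mapped into that moving range, with an offset on the lower bound.
; Second-joint rotation and serial-port sending defer to the parent.
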(fn `enviarPuertoSerie`
  (`parent.enviarPuertoSerie`))

(fn `rotarPrimeraArticulacion`
  (params (Falange1 :type "StaticMeshComponent Object Reference") (angulo :type "Float (double-precision)"))
  (bind _returnvalue (- 0.0 angulo))
  (set `self.minPolea2` (`KismetMathLibrary.MapRangeClamped` _returnvalue 0.0 90.0 30.0 50.0))
  (set `self.maxPolea2` (`KismetMathLibrary.MapRangeClamped` _returnvalue 7.0 70.0 150.0 170.0))
  (`parent.rotarPrimeraArticulacion` Falange1 angulo))

(fn `rotarSegundaArticulacion`
  (params (falange2 :type "StaticMeshComponent Object Reference") (falange3 :type "StaticMeshComponent Object Reference") (angulo :type "Float (double-precision)"))
  (`parent.rotarSegundaArticulacion` falange2 falange3 angulo))

(fn `transformacionFalange2`
  (params (gradosFalange2 :type "Float (double-precision)"))
  (returns (gardosPolea2 :type "Float (double-precision)"))
  (return (`KismetMathLibrary.MapRangeClamped` (- 0.0 gradosFalange2) 7.0 70.0 (+ (`self.desfaseFalange2`) (`self.minPolea2`)) (`self.maxPolea2`))))

(fn `UserConstructionScript`
  (`parent.UserConstructionScript`))